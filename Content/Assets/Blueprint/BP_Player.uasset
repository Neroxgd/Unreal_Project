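; Player Blueprint with camera-relative movement and mouse-driven yaw on an Empty component that serves as the view pivot.
; Each tick, forward/right inputs become a normalized local offset from that pivot's vectors, without sweep or delta-time scaling.
; While moving, the Mesh yaw lerps in 0.1 steps toward a look-at from actor location to the pivot's forward vector, used directly as a target position.
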(event Custom|Move
  (bind _returnvalue (Input|AxisValues|Getgorightleft))
  (bind _returnvalue_2 (Input|AxisValues|Getgoforwardbackward))
  (bind _empty (Variables|Default|Getempty))
  (bind _empty_2 (Variables|Default|Getempty))
  (bind _returnvalue_3 (Math|Vector|GetForwardVector _empty_2))
  (bind _returnvalue_4 (Math|Vector|GetRightVector _empty))
  (bind _returnvalue_5 (* _returnvalue_4 -1.0 _returnvalue))
  (bind _returnvalue_6 (* _returnvalue_3 -1.0 _returnvalue_2))
  (bind _returnvalue_7 (+ _returnvalue_6 _returnvalue_5))
  (bind _returnvalue_8 (Math|Vector|Normalize _returnvalue_7))
  ;[1 1 1] Move
  (Transformation|AddActorLocalOffset _returnvalue_8 false false)
  (if (Utilities|Operators|NotEqual(!=) _returnvalue_8 (Math|Vector|VectorZero) 0.0)
    (Variables|Default|Setlerpf 0.0)
    (Variables|Default|SetrotateTrigger true)))

(event Custom|Rotate
  (if (Variables|Default|GetrotateTrigger)
    (bind _output_get (Variables|Default|Setlerpf (+ (Variables|Default|Getlerpf) 0.1)))
    (Transformation|SetWorldRotation (Variables|Character|GetMesh) (Math|Rotator|MakeRotator 0.0 0.0 (.yaw (Math|Rotator|Lerp(Rotator) (Transformation|GetWorldRotation (Variables|Character|GetMesh)) (Math|Rotator|FindLookatRotation (Transformation|GetActorLocation) (Math|Vector|GetForwardVector (Variables|Default|Getempty))) (Math|Float|Clamp(Float) _output_get)))) false false)
    (Variables|Default|SetrotateTrigger false)
    (Development|PrintString (Utilities|String|ToString(Float) (Variables|Default|Getlerpf)))))

(event EventTick
  (params (DeltaSeconds :type Float%20%28single-precision%29))
  (Utilities|FlowControl|Sequence
    (:then_0
      (CallFunction|Move))
    (:then_1
      (CallFunction|Rotate))))

(event Input|MouseEvents|MouseX
  (params (AxisValue :type Float%20%28single-precision%29))
  ;[1 1 1] Cam
  (Transformation|AddRelativeRotation (Variables|Default|Getempty) (Math|Rotator|MakeRotator 0.0 0.0 AxisValue) false false))

(fn ConstructionScript)